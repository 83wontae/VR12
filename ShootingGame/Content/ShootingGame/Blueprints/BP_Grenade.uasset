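; BP_Grenade is a timed grenade for the shooting game that explodes three seconds after spawning, with the fuse set only on the authority.
; EventExplosion pushes and damages overlapping BP_ShootingCharacters, scaling impulse and damage by linear falloff across the DamageArea radius.
; ResExplosion then spawns the particle effect, disables the sphere's physics and collision, and hides the actor, which is destroyed after a further delay.
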(event Custom|ResExplosion
  (bind _sphere (Variables|Default|GetSphere))
  (Effects|SpawnEmitteratLocation "/Game/StarterContent/Particles/P_Explosion.P_Explosion" (Transformation|GetActorLocation) (Transformation|GetActorRotation) "3.000000,3.000000,3.000000")
  (Physics|SetSimulatePhysics _sphere false)
  (Collision|SetCollisionEnabled _sphere "NoCollision")
  (Rendering|SetActorHiddenInGame true))

(event EventBeginPlay
  (Networking|SwitchHasAuthority
    (:Authority
      (Utilities|Time|SetTimerbyFunctionName 0 "EventExplosion" 3.0))))

(fn ConstructionScript)

(fn EventExplosion
  (CallFunction|ApplyAreaDamage)
  (CallFunction|ResExplosion)
  (Utilities|Time|SetTimerbyFunctionName 0 "DelayDestroy" 3.0))

(fn DelayDestroy
  (Actor|DestroyActor))

(fn ApplyAreaDamage
  (for _array_element (Collision|GetOverlappingActors (Variables|Default|GetDamageArea) "/Game/ShootingGame/GameMode/InGame/BP_ShootingCharacter.BP_ShootingCharacter_C" :!class /Script/Engine.PrimitiveComponent)
    (CallFunction|PushCharacter _array_element)
    (Game|Damage|ApplyDamage _array_element (CallFunction|GetDistanceDamage (Transformation|GetActorLocation _array_element) (Transformation|GetActorLocation)) (Variables|Default|GetInstigatorChar) self)))

(fn GetDistanceDamage
  (params (V1 :type Vector) (V2 :type Vector))
  (return (* (CallFunction|GetDistanceInvPer V1 V2) (Variables|Default|GetBaseDamage))))

(fn PushCharacter
  (params (Char :type Object%20Object%20Reference))
  (bind _returnvalue (Transformation|GetActorLocation))
  (bind _as캐릭터 (Utilities|Casting|CastToCharacter Char))
  (Physics|AddImpulse (Variables|/Script/Engine.Character|GetCharacterMovement _as캐릭터) (* (Math|Vector|GetForwardVector (Math|Rotator|FindLookatRotation _returnvalue (Transformation|GetActorLocation _as캐릭터))) (* (CallFunction|GetDistanceInvPer _returnvalue (Transformation|GetActorLocation _as캐릭터)) 1e+05)) false))

(fn GetDistanceInvPer
  (params (V1 :type Vector) (V2 :type Vector))
  (bind _damagearea (Variables|Default|GetDamageArea))
  (bind _sphereradius (Variables|/Script/Engine.SphereComponent|GetSphereRadius _damagearea))
  (return (/ (- _sphereradius (Math|Vector|Distance(Vector) V1 V2)) _sphereradius)))