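; HUD Blueprint for the shooting game that relays the player's health, ammo and magazine values to the on-screen widget.
; On BeginPlay it runs the parent logic, switches the first player controller to game-only input and hides the mouse cursor.
; Each update event casts HudWidget to ShootingHudWidget and calls the matching setter, doing nothing if the cast fails.
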(event EventBeginPlay
  (bind _returnvalue (Game|GetPlayerController 0))
  (|CallParentFunction)
  (Input|SetInputModeGameOnly _returnvalue true)
  (Variables|/Script/Engine.PlayerController|SetbShowMouseCursor _returnvalue false))

(event EventOnUpdateMyHp
  (params (CurHp :type Float%20%28single-precision%29) (MaxHp :type Float%20%28single-precision%29))
  (bind _asshooting_hud_widget (Utilities|Casting|CastToShootingHudWidget (Variables|Default|GetHudWidget)))
  (Default|SetHp _asshooting_hud_widget CurHp MaxHp))

(event EventOnUpdateMyAmmo
  (params (Ammo :type Integer))
  (bind _asshooting_hud_widget (Utilities|Casting|CastToShootingHudWidget (Variables|Default|GetHudWidget)))
  (Default|SetAmmo _asshooting_hud_widget Ammo))

(event EventOnUpdateMyMag
  (params (Mag :type Integer))
  (bind _asshooting_hud_widget (Utilities|Casting|CastToShootingHudWidget (Variables|Default|GetHudWidget)))
  (Default|SetMag _asshooting_hud_widget Mag))

(fn ConstructionScript)