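; Player state for the shooting game that holds a player's current and maximum health.
; Health starts at the maximum on BeginPlay, and AddDamage and AddHeal adjust it, clamped between zero and that maximum.
; CurHp uses a RepNotify, which fires the UpdateHp event dispatcher with current and maximum values so listeners can react to changes.
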(event EventBeginPlay
  (Variables|Default|SetCurHp (Variables|Default|GetMaxHp)))

(fn ConstructionScript)

(fn AddDamage
  (params (Damage :type Float%20%28double-precision%29))
  (Variables|Default|SetCurHp (Math|Float|Clamp(Float) (- (Variables|Default|GetCurHp) Damage) 0.0 (Variables|Default|GetMaxHp))))

(fn OnRepCurHp
  (Default|CallEventDispatcherUpdateHp (Variables|Default|GetCurHp) (Variables|Default|GetMaxHp)))

(fn AddHeal
  (params (Heal :type Float%20%28double-precision%29))
  (Variables|Default|SetCurHp (Math|Float|Clamp(Float) (+ (Variables|Default|GetCurHp) Heal) 0.0 (Variables|Default|GetMaxHp))))