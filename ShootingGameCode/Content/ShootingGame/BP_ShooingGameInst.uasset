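; Game instance Blueprint for the shooting game that prints server names from session search results for debugging.
; On Init it binds a handler to the FucDeleSearchResult delegate, apparently the auto-generated function that prints "Bind"-prefixed names.
; A separate OnUpdateSearchResult event prints every name with an "Event" prefix, showing which notification path fired.
; The auto-generated function ignores IsFind and returns inside its loop, so it prints only the first result.
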(event EventOnUpdateSearchResult
  (params (SessionResults :type Array%20of%20Blueprint%20Session%20Result%20Structures))
  (for _array_element SessionResults
    (Development|PrintString (Utilities|String|Append "Event ServerName : " (Class|FindSessionsCallbackProxy|GetServerName _array_element)))))

(event EventInit
  (EventDispatchers|BindEventtoFucDeleSearchResult (EventDispatchers|CreateEvent :!event BPShooingGameInstAutoGenFunc)))

(fn BPShooingGameInstAutoGenFunc
  (params (isFind :type Boolean) (SearchResults :type Array%20of%20Blueprint%20Session%20Result%20Structures))
  (for _array_element SearchResults
    (Development|PrintString (Utilities|String|Append "Bind ServerName : " (Class|FindSessionsCallbackProxy|GetServerName _array_element)))
    (return)))