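; Skill component for a shooting game that runs data-table-driven skills, buffs and their cooldowns.
; UseSkill applies Buff-type skills through the target's SkillComponent and records cooldowns on the caster, without checking existing ones.
; Tick counts down one shared array of skill and buff timers, removing expired entries through RemoveBuff.
; Buffs toggle the Invin flag, which gates IsCanDamage and broadcasts ChangeStatus from its OnRep.
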(event EventBeginPlay)

(event EventTick
  (params (DeltaSeconds :type Float%20%28single-precision%29))
  (CallFunction|UpdateCoolTime DeltaSeconds))

(fn UseSkill
  (params (SkillKey :type Name) (Target :type Actor%20Object%20Reference))
  (bind _returnvalue (Utilities|GetDataTableRow "/Game/ShootingGame/Datas/DT_Skill.DT_Skill" SkillKey)
    (:then
      (switch Utilities|FlowControl|Switch|SwitchonEn_SkillType (.SkillType (Utilities|Struct|BreakST_Skill _returnvalue))
        (:NewEnumerator1
          (CallFunction|ApplyBuff (Actor|GetComponentbyClass Target "SkillComponent_C") Target SkillKey (.BuffKey (Utilities|Struct|BreakST_Skill _returnvalue)))
          (bind _returnvalue_2 (Utilities|GetDataTableRow "/Game/ShootingGame/Datas/DT_CoolTime.DT_CoolTime" (.CoolTimeKey (Utilities|Struct|BreakST_Skill _returnvalue)))
            (:then
              (CallFunction|AddCoolTime (Utilities|Struct|MakeST_CoolTImeRef _returnvalue_2 (Utilities|Struct|BreakST_CoolTime _returnvalue_2) SkillKey "None")))))))))

(fn ApplyBuff
  (params (Target :type Actor%20Object%20Reference) (SkillKey :type Name) (BuffKey :type Name))
  (Development|PrintString "Apply Buff")
  (bind _returnvalue (Utilities|GetDataTableRow "/Game/ShootingGame/Datas/DT_Buff.DT_Buff" BuffKey)
    (:then
      ;[1 1 1] CoolTIme 처리
      (Utilities|FlowControl|Sequence
        (:then_0
          (bind _returnvalue_2 (Utilities|GetDataTableRow "/Game/ShootingGame/Datas/DT_CoolTime.DT_CoolTime" (.CoolTimeKey (Utilities|Struct|BreakST_Buff _returnvalue)))
            (:then
              (CallFunction|AddCoolTime (Utilities|Struct|MakeST_CoolTImeRef _returnvalue_2 (Utilities|Struct|BreakST_CoolTime _returnvalue_2) SkillKey BuffKey)))))
        (:then_1
          (switch Utilities|FlowControl|Switch|SwitchonEn_BuffType (.BuffType (Utilities|Struct|BreakST_Buff _returnvalue))
            (:NewEnumerator0
              (Variables|Default|Setinvin true))))))))

(fn AddCoolTime
  (params (stCoolTime :type ST%20Cool%20T%20Ime%20Ref%20Structure))
  (Utilities|Array|Add (Variables|Default|GetCoolTimeArr) stCoolTime))

(fn UpdateCoolTime
  (params (DeltaSeconds :type Float%20%28double-precision%29))
  (bind _cooltimearr (Variables|Default|GetCoolTimeArr))
  (bind _cooltimearr_2 (Variables|Default|GetCoolTimeArr))
  (Utilities|FlowControl|Sequence
    (:then_0
      (if (not (Utilities|Array|IsEmpty _cooltimearr_2))
        (for _index (range 0 (- (Utilities|Array|Length _cooltimearr_2) 1))
          (Utilities|Array|SetArrayElem _cooltimearr _index (Utilities|Struct|MakeST_CoolTImeRef (.stcooltime (Utilities|Array|Get(acopy) _cooltimearr _index)) (- (.curcooltime (Utilities|Array|Get(acopy) _cooltimearr _index)) DeltaSeconds) (.skillkey (Utilities|Array|Get(acopy) _cooltimearr _index)) (.buffkey (Utilities|Array|Get(acopy) _cooltimearr _index)))))))
    (:then_1
      (bind _bremoved (CallFunction|UpdateRemoveCoolTime :!label _label))
      (if _bremoved
        (goto _label)))))

(fn RemoveBuff
  (params (CoolTImeRefIndex :type Integer))
  (bind _cooltimearr (Variables|Default|GetCoolTimeArr))
  (Utilities|FlowControl|Sequence
    (:then_0
      (bind _returnvalue (Utilities|GetDataTableRow "/Game/ShootingGame/Datas/DT_Buff.DT_Buff" (.BuffKey (Utilities|Struct|BreakST_CoolTImeRef (Utilities|Array|Get(acopy) _cooltimearr CoolTImeRefIndex))))
        (:then
          (switch Utilities|FlowControl|Switch|SwitchonEn_BuffType (.BuffType (Utilities|Struct|BreakST_Buff _returnvalue))
            (:NewEnumerator0
              (Variables|Default|Setinvin false))))))
    (:then_1
      (Utilities|Array|RemoveIndex _cooltimearr CoolTImeRefIndex)
      (Development|PrintString "Remove Buff"))))

(fn UpdateRemoveCoolTime
  (for (_array_element _array_index) (Variables|Default|GetCoolTimeArr)
    (if (<= (.CurCoolTime (Utilities|Struct|BreakST_CoolTImeRef _array_element)) 0.0)
      (CallFunction|RemoveBuff _array_index)
      (return true)))
  (return false))

(fn IsCanDamage
  (if (Variables|Default|Getinvin)
    (return false)
    (else
      (return true))))

(fn OnRepInvin
  (Development|PrintString "Apply Invin" true true "(R=0.000000,G=0.660000,B=1.000000,A=1.000000)" 1e+01)
  (Default|CallEventDispatcherChangeStatus (Variables|Default|Getinvin)))